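; BP_FallingPlatform is a platform Blueprint that times how long something stays on it, with no falling behavior implemented yet.
; Collision begin and end overlaps toggle PlayerOnPlatform and reset DurationOnPlatform, without filtering which actor overlaps.
; While the flag is set, Tick accumulates delta time into the duration and prints it as debug output.
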(event `self.Collision.OnComponentBeginOverlap`
  (params (OverlappedComponent :type "PrimitiveComponent Object Reference") (OtherActor :type "Actor Object Reference") (OtherComp :type "PrimitiveComponent Object Reference") (OtherBodyIndex :type Integer) (bFromSweep :type Boolean) (SweepResult :type "HitResult Structure (by ref)"))
  (`KismetSystemLibrary.PrintString` "Hello")
  (set `self.PlayerOnPlatform` true)
  (set `self.DurationOnPlatform` 0.0 :!label _label))

(event `self.Collision.OnComponentEndOverlap`
  (params (OverlappedComponent :type "PrimitiveComponent Object Reference") (OtherActor :type "Actor Object Reference") (OtherComp :type "PrimitiveComponent Object Reference") (OtherBodyIndex :type Integer))
  (set `self.PlayerOnPlatform` false)
  (goto _label))

(event `self.ReceiveTick`
  (params (DeltaSeconds :type "Float (single-precision)"))
  (if (`self.PlayerOnPlatform`)
    (set `self.DurationOnPlatform` (+ DeltaSeconds (`self.DurationOnPlatform`)))
    (`KismetSystemLibrary.PrintString` (`KismetStringLibrary.Conv_DoubleToString` (`self.DurationOnPlatform`)))))

(fn `UserConstructionScript`)