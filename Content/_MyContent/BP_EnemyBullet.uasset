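; BP_EnemyBullet is an enemy projectile actor that flies forward and explodes on contact with the player.
; Tick moves it along its local X axis by BulletSpeed each frame, without delta-time scaling, and a Delay chained after the move destroys it after three seconds.
; Overlapping an actor tagged Player spawns an explosion particle effect, then destroys the bullet after a short delay; no damage is applied here.
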(event `self.ReceiveActorBeginOverlap`
  (params (OtherActor :type "Actor Object Reference"))
  (if (`self.ActorHasTag` OtherActor "Player")
    (`GameplayStatics.SpawnEmitterAtLocation` "/Game/StarterContent/Particles/P_Explosion.P_Explosion" (`self.K2_GetActorLocation`))
    (`KismetSystemLibrary.Delay` 0.2)
    (`self.K2_DestroyActor`)))

(event `self.ReceiveTick`
  (params (DeltaSeconds :type "Float (single-precision)"))
  (`self.K2_AddActorLocalOffset` (`KismetMathLibrary.MakeVector` (`KismetMathLibrary.Conv_IntToDouble` (`self.BulletSpeed`))))
  (`KismetSystemLibrary.Delay` 3.0)
  (`self.K2_DestroyActor`))

(fn `UserConstructionScript`)