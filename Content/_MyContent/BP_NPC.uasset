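; BP_NPC is a non-player character that plays a timed sequence of dialogue lines when an overlapping actor tagged Player arrives.
; UpdateDialogue writes the current string from its dialogue array into the player's BP_ThirdPersonCharacter, advances the index, and re-calls itself after a fixed delay until the array ends.
; A ResetDialogue event restarts the sequence from the first line; the overlap itself does not reset the index.
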(event `self.ReceiveActorBeginOverlap`
  (params (OtherActor :type "Actor Object Reference"))
  (if (`self.ActorHasTag` OtherActor "Player")
    (`self.UpdateDialogue`)))

(event `ResetDialogue`
  (set `self.CurrentDialogue` 0)
  (`self.UpdateDialogue`))

(event `UpdateDialogue`
  (bind _asbp_third_person_character (cast `/Game/ThirdPerson/Blueprints/BP_ThirdPersonCharacter` (`GameplayStatics.GetPlayerCharacter` 0)))
  (set `/Game/ThirdPerson/Blueprints/BP_ThirdPersonCharacter.CurrentDialogueTextt` (`|GetArrayItem` (`self.DialogueOfStringType`) (`self.CurrentDialogue`)) _asbp_third_person_character)
  (set `self.CurrentDialogue` (+ (`self.CurrentDialogue`) 1))
  (`KismetSystemLibrary.Delay` 3.0)
  (if (!= (`self.CurrentDialogue`) (`KismetArrayLibrary.Array_Length` (`self.DialogueOfStringType`)))
    (`self.UpdateDialogue`)))

(fn `UserConstructionScript`)