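; BP_ChasingEnemy is an enemy that chases the player once its PawnSensing component spots a pawn.
; The sighting sets a flag that is never cleared, so every Tick it moves toward player pawn 0 and turns to face it.
; A Hit whose other actor casts to BP_ThirdPersonGameMode launches the enemy along LaunchDirection and decrements Health, destroying it when none remains.
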(event `self.ReceiveTick`
  (params (DeltaSeconds :type "Float (single-precision)"))
  (if (`self.SeesPlayer`)
    (`self.FollowPlayer`)))

(event `self.PawnSensing.OnSeePawn`
  (params (Pawn :type "Pawn Object Reference"))
  (set `self.SeesPlayer` true))

(event `FollowPlayer`
  (bind (_returnvalue_x _returnvalue_y) (`KismetMathLibrary.BreakVector` (`self.K2_GetActorLocation`)))
  (bind (_returnvalue_x_2 _returnvalue_y_2) (`KismetMathLibrary.BreakVector` (`self.K2_GetActorLocation` (`GameplayStatics.GetPlayerPawn` 0))))
  ;[1 1 1] Comment
  (`self.AddMovementInput` (`KismetMathLibrary.Normal` (- (`self.K2_GetActorLocation` (`GameplayStatics.GetPlayerPawn` 0)) (`self.K2_GetActorLocation`) (0.0 0.0 0.0))))
  (`self.K2_SetActorRotation` (`KismetMathLibrary.FindLookAtRotation` (`KismetMathLibrary.MakeVector` _returnvalue_x _returnvalue_y) (`KismetMathLibrary.MakeVector` _returnvalue_x_2 _returnvalue_y_2))))

(event `self.ReceiveHit`
  (params (MyComp :type "PrimitiveComponent Object Reference") (Other :type "Actor Object Reference") (OtherComp :type "PrimitiveComponent Object Reference") (bSelfMoved :type Boolean) (HitLocation :type "Vector Structure") (HitNormal :type "Vector Structure") (NormalImpulse :type "Vector Structure") (Hit :type "HitResult Structure (by ref)"))
  (cast `/Game/ThirdPerson/Blueprints/BP_ThirdPersonGameMode` Other)
  (`self.LaunchCharacter` (`self.LaunchDirection`))
  (set `self.Health` (- (`self.Health`) 1))
  (if (<= (`self.Health`) 0)
    (`self.K2_DestroyActor`)))

(fn `UserConstructionScript`)