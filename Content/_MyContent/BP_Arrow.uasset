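; Arrow actor that flies along its local Z axis, moved by ArrowSpeed every Tick without delta-time scaling.
; On Box overlap, unless the arrow itself is tagged "Socket", it attaches to the swept hit component, keeping world rotation, and prints a debug message.
; Nothing here stops the Tick movement after attaching.
; Line-trace nodes for hit location, normal and bone are unconnected and never run.
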(event `self.ReceiveTick`
  (params (DeltaSeconds :type "Float (single-precision)"))
  (`self.K2_AddActorLocalOffset` (`KismetMathLibrary.MakeVector` 0.0 0.0 (`KismetMathLibrary.Conv_IntToDouble` (`self.ArrowSpeed`)))))

(event `self.Box.OnComponentBeginOverlap`
  (params (OverlappedComponent :type "PrimitiveComponent Object Reference") (OtherActor :type "Actor Object Reference") (OtherComp :type "PrimitiveComponent Object Reference") (OtherBodyIndex :type Integer) (bFromSweep :type Boolean) (SweepResult :type "HitResult Structure (by ref)"))
  (if (not (`self.ActorHasTag` "Socket"))
    (`self.K2_AttachToComponent` (`.HitComponent` (`GameplayStatics.BreakHitResult` SweepResult)) "None" "KeepRelative" "KeepWorld" "KeepRelative")
    (`KismetSystemLibrary.PrintString` "set")))

(fn `UserConstructionScript`)