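; Enemy turret that fires continuously from BeginPlay, either single arrows or scattered bullet bursts depending on IsScatterShot.
; Shoot and ScatterShot re-call themselves after a FiringRate delay, spawning projectiles at SMFiringPoint, with random yaw spread for scatter.
; When LookAtPlayer is set, Tick turns the turret toward the player and snaps it to the player's height.
; VerticalFiring scales the Z values used for aiming.
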(event `self.ReceiveTick`
  (params (DeltaSeconds :type "Float (single-precision)"))
  (`self.FollowPlayer`))

(event `self.ReceiveBeginPlay`
  (if (`self.IsScatterShot`)
    (`self.ScatterShot`)
    (else
      (`self.Shoot`))))

(event `Shoot`
  (`|SpawnActorFromClass` "/Game/_MyContent/BP_Arrow.BP_Arrow_C" (`SceneComponent.GetSocketTransform` (`self.SM_FiringPoint`) "None" "RTS_World") "Undefined" "MultiplyWithRoot" null null)
  (`KismetSystemLibrary.Delay` (`self.FiringRate`))
  (`self.Shoot`))

(event `FollowPlayer`
  (bind (_returnvalue_x _returnvalue_y _returnvalue_z) (`KismetMathLibrary.BreakVector` (`self.K2_GetActorLocation`)))
  (bind (_returnvalue_x_2 _returnvalue_y_2) (`KismetMathLibrary.BreakVector` (`self.K2_GetActorLocation`)))
  (bind (_returnvalue_x_3 _returnvalue_y_3 _returnvalue_z_2) (`KismetMathLibrary.BreakVector` (`self.K2_GetActorLocation` (`GameplayStatics.GetPlayerPawn` 0))))
  (bind (_returnvalue_x_4 _returnvalue_y_4 _returnvalue_z_3) (`KismetMathLibrary.BreakVector` (`self.K2_GetActorLocation` (`GameplayStatics.GetPlayerPawn` 0))))
  ;[1 1 1] Comment
  (if (`self.LookAtPlayer`)
    (`self.K2_SetActorRotation` (`KismetMathLibrary.FindLookAtRotation` (`KismetMathLibrary.MakeVector` _returnvalue_x _returnvalue_y (* _returnvalue_z (`self.VerticalFiring`))) (`KismetMathLibrary.MakeVector` _returnvalue_x_3 _returnvalue_y_3 (* _returnvalue_z_2 (`self.VerticalFiring`)))))
    (`self.K2_SetActorLocation` (`KismetMathLibrary.MakeVector` _returnvalue_x_2 _returnvalue_y_2 _returnvalue_z_3))))

(event `ScatterShot`
  (bind _returnvalue (`SceneComponent.GetSocketTransform` (`self.SM_FiringPoint`) "None" "RTS_World"))
  ;[1 1 1] Comment
  (for _ (range 3)
    (`|SpawnActorFromClass` "/Game/_MyContent/BP_EnemyBullet.BP_EnemyBullet_C" (`KismetMathLibrary.MakeTransform` (.location _returnvalue) (`KismetMathLibrary.MakeRotator` (.roll (.rotation _returnvalue)) (.pitch (.rotation _returnvalue)) (+ (.yaw (.rotation _returnvalue)) (`KismetMathLibrary.RandomFloatInRange` -30.0 30.0)))) "Undefined" "MultiplyWithRoot" null null))
  (`KismetSystemLibrary.Delay` (`self.FiringRate`))
  (`self.ScatterShot`))

(fn `UserConstructionScript`)